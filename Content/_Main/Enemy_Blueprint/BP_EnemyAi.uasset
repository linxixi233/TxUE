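; Enemy AI character that chases the player on sight and dies when shot.
; Pawn sensing triggers an AI move toward the player, then plays a rifle-shoot montage on arrival, gated by a flag until the montage ends; no damage is applied here.
; A capsule hit from an actor tagged Bullet enables mesh physics for a ragdoll, clears the alive flag and disables capsule collision.
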(event `self.PawnSensing.OnSeePawn`
  (params (Pawn :type "Pawn Object Reference"))
  (set `self.isSeeingPlayer?` true)
  (`self.FollowPlayer`))

(event `FollowPlayer`
  (set `self.canAttack?` true)
  (if (`self.isSeeingPlayer?`)
    (`|AIMoveTo` self (0.0 0.0 0.0) (`GameplayStatics.GetPlayerCharacter` 0) 72.0
      (:`OnSuccess`
        (if (`self.canAttack?`)
          (set `self.canAttack?` false)
          (bind _returnvalue (`self.PlayAnimMontage` "/Game/FirstPersonArms/Animations/FP_Rifle_Shoot_Montage.FP_Rifle_Shoot_Montage"))
          (`KismetSystemLibrary.Delay` _returnvalue)
          (set `self.canAttack?` true))))))

(event `self.CapsuleComponent.OnComponentHit`
  (params (HitComponent :type "PrimitiveComponent Object Reference") (OtherActor :type "Actor Object Reference") (OtherComp :type "PrimitiveComponent Object Reference") (NormalImpulse :type "Vector Structure") (Hit :type "HitResult Structure (by ref)"))
  (if (`self.ActorHasTag` OtherActor "Bullet")
    (`self.Ragdoll`)))

(event `Ragdoll`
  (bind _mesh (`self.Mesh`))
  (if (`self.isAlive?`)
    (`PrimitiveComponent.SetCollisionEnabled` _mesh "QueryAndPhysics")
    (`PrimitiveComponent.SetSimulatePhysics` _mesh true)
    (`SkeletalMeshComponent.SetPhysicsBlendWeight` _mesh 0.0)
    (set `self.isAlive?` false)
    (`PrimitiveComponent.SetCollisionEnabled` (`self.CapsuleComponent`) "NoCollision")))

(fn `UserConstructionScript`)