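; Base weapon pickup actor that gives an interacting character a weapon and then removes itself from the world.
; On Interact, it adds a WeaponToSpawn component to that character, snaps it to the AR_B_Socket socket on the first-person mesh, and destroys the pickup.
; GetWeaponClass returns a separate WeaponClass variable, which the Interact logic does not use.
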(event `/Game/_Main/interfaces/BPI_Interact.Interact`
  (params (`Chracter Picking Up` :type "/Game/FirstPerson/Blueprints/BP_FirstPersonCharacter Object Reference"))
  (bind _returnvalue (`|AddComponentByClass` :`self` `Chracter Picking Up` :`Class` (`self.Weapon To Spawn`)))
  (`SceneComponent.K2_AttachToComponent` _returnvalue (`/Game/FirstPerson/Blueprints/BP_FirstPersonCharacter.FirstPersonMesh` `Chracter Picking Up`) "AR_B_Socket" "SnapToTarget" "SnapToTarget" "KeepRelative" true)
  (`self.K2_DestroyActor`))

(fn `Get Weapon Class`
  (returns (`Pickup Weapon Class` :type "/Game/_Main/props/Weapons/Enum_WeaponClass Enum"))
  (return (`self.Weapon Class`)))

(fn `UserConstructionScript`
  (`parent.UserConstructionScript`))