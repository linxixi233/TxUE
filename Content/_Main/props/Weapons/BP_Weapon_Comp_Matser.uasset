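; Master weapon component for the first-person character, with a graph for equipping itself into a primary or secondary slot.
; The logic replaces any weapon in its class's slot, marks itself equipped and stores its weapon name as the character's weapon index.
; It then snaps to a socket on the first-person mesh for local players, or the third-person body otherwise.
; BeginPlay is empty and nothing triggers this chain, so it never runs.
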(event `self.ReceiveBeginPlay`)